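; Door Blueprint that reacts to a multi-plate puzzle and swings open when the puzzle is solved.
; Wrong and correct plate events play an explosion or lock sound at the door.
; The solved event runs the DoorSwing timeline, which adds yaw to InitialRotation and retriggers the lock sound on a timed track.
; The node capturing InitialRotation from the actor is disconnected, so that assignment never runs.
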(event `self.MultiPlatePuzzle.OnWrongPlate`
  (`GameplayStatics.SpawnSoundAtLocation` "/Game/StarterContent/Audio/Explosion01.Explosion01" (`self.K2_GetActorLocation`)))

(event `self.MultiPlatePuzzle.OnCorrectPlate`
  (`GameplayStatics.SpawnSoundAtLocation` "/Game/Audio/door-lock.door-lock" (`self.K2_GetActorLocation`)))

(event `self.MultiPlatePuzzle.OnSolved`
  (bind (_direction _open_angle) (`Timeline|Door Swing`)
    (:`Update`
      (`self.K2_SetActorRotation` (`KismetMathLibrary.ComposeRotators` (`KismetMathLibrary.MakeRotator` 0.0 0.0 _open_angle) (`self.Initial Rotation`))) ; Open the door.
    )
    (:`Sound Timing`
      (`GameplayStatics.SpawnSoundAtLocation` "/Game/Audio/door-lock.door-lock" (`self.K2_GetActorLocation`)))))

(fn `UserConstructionScript`)