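; Sliding wall actor that acts as a door, moving vertically when the OpenDoor open and close events fire.
; BeginPlay caches the starting location.
; OnOpen plays the DoorSlide timeline and OnClose reverses it, with each update setting the location to the start plus the curve's Z offset, without sweep.
; A timeline event track spawns the Doorlock sound at the starting location.
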(event `self.OpenDoor.OnOpen`
  (bind (_direction _slide_distance) (`Timeline|Door Slide` :!label _label)
    (:`Update`
      (`self.K2_SetActorLocation` (+ (`KismetMathLibrary.MakeVector` 0.0 0.0 _slide_distance) (`self.InitialLocation`))))
    (:`Sound Timing`
      (`GameplayStatics.SpawnSoundAtLocation` "/Game/Audio/door-lock.door-lock" (`self.InitialLocation`)))))

(event `self.OpenDoor.OnClose`
  (goto _label :!via `Reverse`))

(event `self.ReceiveBeginPlay`
  ;[1 1 1] Get the initial location of the door.
  (set `self.InitialLocation` (`self.K2_GetActorLocation`)))

(fn `UserConstructionScript`)